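; Base pickup actor that flies toward the player and destroys itself when collected.
; Overlapping ColliderRange starts the MoveToPlayer timeline, which interpolates the actor toward the player's location at MoveSpeed, adding the timeline's MovementTrack as an offset.
; Player overlap with ItemCollider calls OnItemPickup, an empty event that serves as a hook for item effects, then destroys the actor.
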(event OnComponentBeginOverlap(ColliderRange)
  (params (OverlappedComponent :type Primitive%20Component%20Object%20Reference) (OtherActor :type Actor%20Object%20Reference) (OtherComp :type Primitive%20Component%20Object%20Reference) (OtherBodyIndex :type Integer) (bFromSweep :type Boolean) (SweepResult :type Hit%20Result%20Structure%20%28by%20ref%29))
  (bind _returnvalue (Game|GetPlayerCharacter 0))
  (if (== OtherActor _returnvalue)
    (bind _movementtrack (Timeline|MoveToPlayer PlayFromStart)
      (:Update
        (Transformation|SetActorLocation (+ _movementtrack (Math|Interpolation|VInterpTo (.Location (Math|Transform|BreakTransform (Transformation|GetActorTransform))) (Transformation|GetActorLocation _returnvalue) (Utilities|Time|GetWorldDeltaSeconds) (Variables|Default|GetMoveSpeed))) false false)))))

(event OnComponentBeginOverlap(ItemCollider)
  (params (OverlappedComponent :type Primitive%20Component%20Object%20Reference) (OtherActor :type Actor%20Object%20Reference) (OtherComp :type Primitive%20Component%20Object%20Reference) (OtherBodyIndex :type Integer) (bFromSweep :type Boolean) (SweepResult :type Hit%20Result%20Structure%20%28by%20ref%29))
  (if (== OtherActor (Game|GetPlayerCharacter 0))
    (CallFunction|OnItemPickup)
    (Actor|DestroyActor)))

(event Custom|OnItemPickup)

(event EventBeginPlay)

(event Collision|EventActorBeginOverlap
  (params (OtherActor :type Actor%20Object%20Reference)))

(event EventTick
  (params (DeltaSeconds :type Float%20%28single-precision%29)))

(fn ConstructionScript)