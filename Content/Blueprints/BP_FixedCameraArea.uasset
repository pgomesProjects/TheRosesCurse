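; BP_FixedCameraArea is a trigger volume that switches the player to a fixed camera while they are inside it.
; When a PlayerCharacter enters the Collider, the player controller blends its view to FixedCamera over BlendTime and the character's CurrentCameraAngle takes the area's CameraAngle.
; On exit, the view blends back to the character's PlayerCamera and the angle resets to the enum's NewEnumerator0 entry.
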(event OnComponentBeginOverlap(Collider)
  (params (OverlappedComponent :type Primitive%20Component%20Object%20Reference) (OtherActor :type Actor%20Object%20Reference) (OtherComp :type Primitive%20Component%20Object%20Reference) (OtherBodyIndex :type Integer) (bFromSweep :type Boolean) (SweepResult :type Hit%20Result%20Structure%20%28by%20ref%29))
  (bind _asplayer_character (Utilities|Casting|CastToPlayerCharacter OtherActor))
  (Game|Player|SetViewTargetwithBlend (Game|GetPlayerController 0) (Variables|Default|GetFixedCamera) (Variables|Default|GetBlendTime) "VTBlend_Linear" 0.0 false)
  (Variables|/Game/Characters/Player/PlayerCharacter.PlayerCharacter_C|SetCurrentCameraAngle _asplayer_character (Variables|Default|GetCameraAngle)))

(event OnComponentEndOverlap(Collider)
  (params (OverlappedComponent :type Primitive%20Component%20Object%20Reference) (OtherActor :type Actor%20Object%20Reference) (OtherComp :type Primitive%20Component%20Object%20Reference) (OtherBodyIndex :type Integer))
  (bind _asplayer_character (Utilities|Casting|CastToPlayerCharacter OtherActor))
  (Game|Player|SetViewTargetwithBlend (Game|GetPlayerController 0) (Variables|/Game/Characters/Player/PlayerCharacter.PlayerCharacter_C|GetPlayerCamera _asplayer_character) (Variables|Default|GetBlendTime) "VTBlend_Linear" 0.0 false)
  (Variables|/Game/Characters/Player/PlayerCharacter.PlayerCharacter_C|SetCurrentCameraAngle _asplayer_character "NewEnumerator0"))

(event EventBeginPlay)

(event Collision|EventActorBeginOverlap
  (params (OtherActor :type Actor%20Object%20Reference)))

(event EventTick
  (params (DeltaSeconds :type Float%20%28single-precision%29)))

(fn ConstructionScript)