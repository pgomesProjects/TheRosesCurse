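; Stair actor that carries the 2D player character from Floor 01 to Floor 02 when it overlaps the lower-floor trigger.
; It locks movement and freezes the camera, slides the player to the stair point, then teleports to the upper floor.
; The camera moves to the exit while the player slides out, then control is restored.
; A timeline-driven lerp with duration-scaled play rate handles both slides.
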(event OnComponentBeginOverlap(Floor01StairsTrigger_CollisionComp)
  (params (OverlappedComponent :type Primitive%20Component%20Object%20Reference) (OtherActor :type Actor%20Object%20Reference) (OtherComp :type Primitive%20Component%20Object%20Reference) (OtherBodyIndex :type Integer) (bFromSweep :type Boolean) (SweepResult :type Hit%20Result%20Structure%20%28by%20ref%29))
  (bind _stairmovementtime (Variables|Default|GetStairMovementTime))
  (bind _stairmovementtime_2 (Variables|Default|GetStairMovementTime))
  (bind _floor02end_defaultsceneroot (Variables|Default|GetFloor02End_DefaultSceneRoot))
  (bind _returnvalue (Transformation|GetWorldLocation _floor02end_defaultsceneroot))
  (bind _as2dplayer_character (Utilities|Casting|CastTo2DPlayerCharacter OtherActor))
  (Variables|Default|SetPlayerRef _as2dplayer_character)
  (if (not (Variables|Default|GetTransitionActive?))
    (Variables|Default|SetTransitionActive? true)
    (Pawn|Components|CharacterMovement|DisableMovement (Variables|/Script/Engine.Character|GetCharacterMovement (Variables|Default|GetPlayerRef)))
    (Components|Movement|StopMovementImmediately (Variables|/Script/Engine.Character|GetCharacterMovement (Variables|Default|GetPlayerRef)))
    (Variables|/Game/Characters/Player/BP_PlayerCamera.BP_PlayerCamera_C|SetCameraFrozen? (Variables|/Game/Characters/Player/2DPlayerCharacter.2DPlayerCharacter_C|GetPlayerCamera (Variables|Default|GetPlayerRef)) true)
    (CallFunction|MovePlayertoLocation (Transformation|GetActorLocation (Variables|Default|GetPlayerRef)) (Transformation|GetWorldLocation (Variables|Default|GetFloor01Stairs_DefaultSceneRoot)) _stairmovementtime)
    (Utilities|FlowControl|Delay _stairmovementtime)
    (Transformation|SetActorLocation (Variables|Default|GetPlayerRef) (Transformation|GetWorldLocation (Variables|Default|GetFloor02Stairs_DefaultSceneRoot)) false true)
    (Default|MoveCamera (Variables|/Game/Characters/Player/2DPlayerCharacter.2DPlayerCharacter_C|GetPlayerCamera (Variables|Default|GetPlayerRef)) _returnvalue (Variables|Default|GetCameraMovementSpeed))
    (CallFunction|MovePlayertoLocation (Transformation|GetWorldLocation (Variables|Default|GetFloor02Stairs_DefaultSceneRoot)) _returnvalue _stairmovementtime_2)
    (Utilities|FlowControl|Delay _stairmovementtime_2)
    (Variables|Default|SetTransitionActive? false)
    (Pawn|Components|CharacterMovement|SetMovementMode (Variables|/Script/Engine.Character|GetCharacterMovement (Variables|Default|GetPlayerRef)) "MOVE_Walking" 0)
    (Variables|/Game/Characters/Player/BP_PlayerCamera.BP_PlayerCamera_C|SetCameraFrozen? (Variables|/Game/Characters/Player/2DPlayerCharacter.2DPlayerCharacter_C|GetPlayerCamera (Variables|Default|GetPlayerRef)) false)))

(event Custom|MovePlayerToLocation
  (params (StartPosition :type Vector) (EndPosition :type Vector) (Seconds :type Float%20%28single-precision%29))
  (Components|Timeline|SetPlayRate (Variables|Default|GetMovePlayerTimeline) (/ 1.0 Seconds))
  (bind _alpha (Timeline|MovePlayerTimeline PlayFromStart)
    (:Update
      (Transformation|SetActorLocation (Variables|Default|GetPlayerRef) (Math|Vector|Lerp(Vector) StartPosition EndPosition _alpha) false false))))

(event EventBeginPlay)

(event Collision|EventActorBeginOverlap
  (params (OtherActor :type Actor%20Object%20Reference)))

(event EventTick
  (params (DeltaSeconds :type Float%20%28single-precision%29)))

(fn ConstructionScript)